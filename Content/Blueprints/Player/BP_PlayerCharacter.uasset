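; BP_PlayerCharacter is the player character Blueprint, routing input into the Gameplay Ability System.
; Primary attack, Q and E press ability input IDs, while R, or a held attack when a checked attribute hits zero, activates GA_WeaponReload.
; A locally controlled character creates the WBP_Gameplay widget on controller change and removes it when destroyed.
; A helper supplies the projectile spawn location and rotation from an arrow component.
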(event Custom|ReloadWeapon
  (Abilities|TryActivateAbilitybyClass (Variables|Default|GetPCAbilitySystemComponent) "/Game/Blueprints/Abilities/Weapon/GA_WeaponReload.GA_WeaponReload_C" true))

(event Custom|OnDestroyed_Event
  (params (DestroyedActor :type Actor%20Object%20Reference))
  (bind _gameplayui (Variables|Default|GetGameplayUI)
    (:then
      (Widget|RemovefromParent _gameplayui))
    (:else)))

(event Input|EnhancedActionEvents|EnhancedInputActionIA_PrimaryAttack
  (params (ActionValue :type Boolean) (ElapsedSeconds :type Float%20%28double-precision%29) (TriggeredSeconds :type Float%20%28double-precision%29) (InputAction :type Input%20Action%20Object%20Reference :default "/Game/Blueprints/Inputs/IA_PrimaryAttack.IA_PrimaryAttack"))
  (bind _pcabilitysystemcomponent (Variables|Default|GetPCAbilitySystemComponent))
  ;[1 1 1] Needs proper Queue system
  (:Started
    (Class|AbilitySystemComponent|PressInputID _pcabilitysystemcomponent 1))
  (:Ongoing
    (if (== (.ReturnValue (Class|AbilitySystemComponent|GetGameplayAttributeValue _pcabilitysystemcomponent "(AttributeName=\"Ammo\",Attribute=/Script/PerfectCity.PCWeaponAttributeSet:Ammo,AttributeOwner=\"/Script/CoreUObject.Class'/Script/PerfectCity.PCWeaponAttributeSet'\")")) 0.0)
      (CallFunction|ReloadWeapon)))
  (:Completed
    (Class|AbilitySystemComponent|ReleaseInputID _pcabilitysystemcomponent 1)))

(event EventBeginPlay
  (|CallParentFunction)
  (Game|AssignOnDestroyed (delegate Custom|OnDestroyed_Event)))

(event EventControllerChanged
  (params (OldController :type Controller%20Object%20Reference) (NewController :type Controller%20Object%20Reference))
  (Utilities|FlowControl|Delay 0.0)
  (if (Pawn|IsLocallyControlled)
    (Variables|Default|GetGameplayUI
      (:then)
      (:else
        (bind _returnvalue (UserInterface|CreateWidget "/Game/Blueprints/UI/WBP_Gameplay.WBP_Gameplay_C" (Game|GetPlayerController 0)))
        (bind _output_get (Variables|Default|SetGameplayUI _returnvalue))
        (UserInterface|Viewport|AddtoViewport _output_get 0)))))

(event Input|KeyboardEvents|R
  (params (Key :type Key%20Structure :default "None"))
  (:Pressed
    (CallFunction|ReloadWeapon)))

(event Input|KeyboardEvents|Q
  (params (Key :type Key%20Structure :default "None"))
  (:Pressed
    (Class|AbilitySystemComponent|PressInputID (Variables|Default|GetPCAbilitySystemComponent) 3)))

(event Input|KeyboardEvents|E
  (params (Key :type Key%20Structure :default "None"))
  (:Pressed
    (Class|AbilitySystemComponent|PressInputID (Variables|Default|GetPCAbilitySystemComponent) 4)))

(fn ConstructionScript)

(fn ProjectileSpawnLocationRotation
  (bind _arrow2 (Variables|Default|GetArrow2))
  (bind _returnvalue (Transformation|GetWorldTransform _arrow2))
  (return (.location _returnvalue) (.rotation _returnvalue)))