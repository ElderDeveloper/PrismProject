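; BP_SkeletonBow is a bow-wielding skeleton monster Blueprint that supplies the spawn transform for its projectiles.
; ProjectileSpawnLocationRotation returns the Arrow1 component's world location, rotated to look at the target actor's location.
; Without a valid target, the rotation follows Arrow1's forward vector.
; The event graph has no active logic, and the construction script only calls the parent.
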(event EventBeginPlay)

(event Collision|EventActorBeginOverlap
  (params (OtherActor :type Actor%20Object%20Reference)))

(event EventTick
  (params (DeltaSeconds :type Float%20%28single-precision%29)))

(fn ConstructionScript
  (|CallParentFunction))

(fn ProjectileSpawnLocationRotation
  (bind _returnvalue (Class|PCAICharacterBase|GetTargetActor))
  (bind _arrow1 (Variables|Default|GetArrow1))
  (bind _returnvalue_2 (Transformation|GetWorldLocation _arrow1))
  (Utilities|IsValid _returnvalue
    (:Is%20Valid
      (return _returnvalue_2 (Math|Rotator|FindLookatRotation _returnvalue_2 (Transformation|GetActorLocation _returnvalue))))
    (:Is%20Not%20Valid
      (return _returnvalue_2 (Math|Rotator|MakeRotfromX (Math|Vector|GetForwardVector _arrow1))))))