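; BP_WeaponBullet is a weapon projectile that applies damage through the Gameplay Ability System.
; Each Tick it sphere-traces on Visibility from its last position to the current one, ignoring its owner, to catch hits along the path.
; A hit applies GE_ApplyDamage with the hit result in the owner's effect context if the target has an Ability System Component, then destroys the bullet regardless.
; The component hit event only prints the impact point.
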(event OnComponentHit(Sphere)
  (params (HitComponent :type Primitive%20Component%20Object%20Reference) (OtherActor :type Actor%20Object%20Reference) (OtherComp :type Primitive%20Component%20Object%20Reference) (NormalImpulse :type Vector :default "0, 0, 0") (Hit :type Hit%20Result%20Structure%20%28by%20ref%29))
  (if (!= OtherActor (Components|GetOwner))
    (Development|PrintString (Utilities|String|ToString(Vector) (.ImpactPoint (Collision|BreakHitResult Hit))) true true "(R=50.000000,G=2.992308,B=0.000000,A=1.000000)")))

(event OnComponentBeginOverlap(Sphere)
  (params (OverlappedComponent :type Primitive%20Component%20Object%20Reference) (OtherActor :type Actor%20Object%20Reference) (OtherComp :type Primitive%20Component%20Object%20Reference) (OtherBodyIndex :type Integer) (bFromSweep :type Boolean) (SweepResult :type Hit%20Result%20Structure%20%28by%20ref%29)))

(event EventTick
  (params (DeltaSeconds :type Float%20%28single-precision%29))
  (bind (_outhit _returnvalue) (Collision|SphereTraceByChannel (Variables|Default|GetCurrentLocation) (Transformation|GetActorLocation) (Components|Sphere|GetScaledSphereRadius (Variables|Default|GetSphere)) "TraceTypeQuery1" false (Utilities|Array|MakeArray (Components|GetOwner)) "None"))
  (if _returnvalue
    (CallFunction|ApplyGameplayEffect _outhit (Ability|GetAbilitySystemComponent (Components|GetOwner)))
    (else
      (Variables|Default|SetCurrentLocation (Transformation|GetActorLocation)))))

(event EventBeginPlay
  (Variables|Default|SetCurrentLocation (Transformation|GetActorLocation)))

(fn ConstructionScript)

(fn ApplyGameplayEffect
  (params (HitResult :type Hit%20Result%20Structure) (OwnerAbility :type Ability%20System%20Component%20Object%20Reference))
  (bind _hitactor (Collision|BreakHitResult HitResult))
  (bind _returnvalue (Ability|GetAbilitySystemComponent _hitactor))
  (Utilities|IsValid _returnvalue
    (:Is%20Valid
      (LocalVariables|SetTargetAbility _returnvalue)
      (bind _output_get (Variables|Default|SetEffectContext (GameplayEffects|MakeEffectContext OwnerAbility)))
      (Class|AbilitySystemBlueprintLibrary|EffectContextAddHitResult _output_get HitResult false)
      (GameplayEffects|ApplyGameplayEffectSpecToTarget OwnerAbility (GameplayEffects|MakeOutgoingSpec (LocalVariables|GetTargetAbility) "/Game/Blueprints/Abilities/GameplayEffects/GE_ApplyDamage.GE_ApplyDamage_C" 1.0 (Variables|Default|GetEffectContext)) (LocalVariables|GetTargetAbility))
      (Actor|DestroyActor))
    (:Is%20Not%20Valid
      (Actor|DestroyActor))))