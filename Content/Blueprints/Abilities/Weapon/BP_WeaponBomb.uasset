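; BP_WeaponBomb is a timed ability bomb that damages nearby PCAICharacterBase characters through the Gameplay Ability System.
; A timer started on BeginPlay activates the explosion effect and runs a Visibility multi-sphere trace at the bomb's location.
; Each character hit receives DamageEffect once, applied from the owner's ability system component with the hit result in its context.
; The bomb destroys itself after a delay, but only when the trace reports a hit.
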(event Custom|CustomEvent
  (bind _returnvalue (Transformation|GetActorLocation))
  (Components|Activation|Activate (Variables|Default|GetExplosion) true)
  (bind (_outhits _returnvalue_2) (Collision|MultiSphereTraceByChannel _returnvalue _returnvalue (Variables|Default|GetExplosionRadius) "TraceTypeQuery1" false 0 "None"))
  (if _returnvalue_2
    (for _array_element _outhits
      (CallFunction|ApplyAreaDamageEffect (.HitActor (Collision|BreakHitResult _array_element)) _array_element))
    (Utilities|FlowControl|Delay 5.0)
    (Actor|DestroyActor)))

(event EventBeginPlay
  (Utilities|Time|SetTimerbyEvent (delegate Custom|CustomEvent) 2.0))

(event Collision|EventActorBeginOverlap
  (params (OtherActor :type Actor%20Object%20Reference)))

(event EventTick
  (params (DeltaSeconds :type Float%20%28single-precision%29)))

(fn ConstructionScript)

(fn ApplyAreaDamageEffect
  (params (Object :type Object%20Object%20Reference) (HitResult :type Hit%20Result%20Structure))
  (bind _returnvalue (Components|GetOwner))
  (bind _returnvalue_2 (Ability|GetAbilitySystemComponent _returnvalue))
  (bind _aspcaicharacter_base (Utilities|Casting|CastToPCAICharacterBase Object))
  (if (== (Utilities|Array|FindItem (Variables|Default|GetDamagedActors) _aspcaicharacter_base) -1)
    (Utilities|Array|Add (Variables|Default|GetDamagedActors) _aspcaicharacter_base)
    (bind _output_get (LocalVariables|SetLocalDamagedActor _aspcaicharacter_base))
    (bind _output_get_2 (LocalVariables|SetEffect (GameplayEffects|MakeEffectContext _returnvalue_2)))
    (Class|AbilitySystemBlueprintLibrary|EffectContextAddHitResult _output_get_2 HitResult false)
    (GameplayEffects|ApplyGameplayEffectToTarget _returnvalue_2 (Variables|Default|GetDamageEffect) (Ability|GetAbilitySystemComponent _output_get) 1.0 (LocalVariables|GetEffect))))